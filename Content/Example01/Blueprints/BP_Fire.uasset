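; BP_Fire is a fire actor in red and blue variants that sets flammable actors alight when they overlap its sphere.
; The IsBlueFire flag picks the particle template in the construction script and selects the overlap branch.
; Each branch checks the overlapping actor for the matching color's BPI_Flammable interface and sends its flame-on message, with a debug print on the blue path.
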(event `self.Sphere.OnComponentBeginOverlap`
  (params (OverlappedComponent :type "PrimitiveComponent Object Reference") (OtherActor :type "Actor Object Reference") (OtherComp :type "PrimitiveComponent Object Reference") (OtherBodyIndex :type Integer) (bFromSweep :type Boolean) (SweepResult :type "HitResult Structure (by ref)"))
  (set `self.Temp_StoredActor` OtherActor)
  (if (`self.bIsBlueFire?`)
    (if (`KismetSystemLibrary.DoesImplementInterface` (`self.Temp_StoredActor`) "/Game/Example01/Blueprints/BPI_Flammable_Blue.BPI_Flammable_Blue_C")
      (message `/Game/Example01/Blueprints/BPI_Flammable_Blue.FlameOn_Blue` (`self.Temp_StoredActor`))
      (`KismetSystemLibrary.PrintString` "Hello"))
    (elif (`KismetSystemLibrary.DoesImplementInterface` (`self.Temp_StoredActor`) "/Game/Example01/Blueprints/BPI_Flammable_Red.BPI_Flammable_Red_C")
      (message `/Game/Example01/Blueprints/BPI_Flammable_Red.FlameOn_Red` (`self.Temp_StoredActor`)))))

(fn `UserConstructionScript`
  (`ParticleSystemComponent.SetTemplate` (`self.ParticleSystem`) (select `bool` (`self.bIsBlueFire?`) :`false` "/Game/Example01/Particles/P_Fire_Red.P_Fire_Red" :`true` "/Game/Example01/Particles/P_Fire_Blue.P_Fire_Blue" :!type "ParticleSystem Object Reference")))