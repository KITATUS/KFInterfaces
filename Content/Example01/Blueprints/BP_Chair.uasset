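; BP_Chair is a chair actor that can be set on fire with either blue or red flames.
; Two events, FlameonBlue and FlameonRed, each activate their matching particle system.
; A shared IsBurning flag lets only the first call take effect, and nothing in these graphs clears it, so the chair keeps that colour.
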(event `/Game/Example01/Blueprints/BPI_Flammable_Blue.FlameOn_Blue`
  (if (not (`self.bIsBurning`))
    (set `self.bIsBurning` true)
    (`ActorComponent.Activate` (`self.ParticleSystem_Blue`) true)))

(event `/Game/Example01/Blueprints/BPI_Flammable_Red.FlameOn_Red`
  (if (not (`self.bIsBurning`))
    (set `self.bIsBurning` true)
    (`ActorComponent.Activate` (`self.ParticleSystem_Red`) true)))

(fn `UserConstructionScript`)