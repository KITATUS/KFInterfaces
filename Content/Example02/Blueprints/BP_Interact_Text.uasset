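; BP_Interact_Text is an example interactable actor that shows its interaction state with text components.
; Its sphere's overlap events message the overlapping actor that it entered or left the zone, and switch an in-volume label between green YES and red NO.
; Each InteractRequest event increments a counter and updates a second text with the number of times it has been interacted with.
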(event `self.ReceiveBeginPlay`
  (`TextRenderComponent.K2_SetText` (`self.Txt_InVolume`) "NO")
  (`TextRenderComponent.SetTextRenderColor` (`self.Txt_InVolume`) (make `Color` 0 0 255)))

(event `self.InteractRequest`
  (params (InteractableActor :type "Actor Object Reference"))
  (`/Engine/EditorBlueprintResources/StandardMacros.IncrementInt` (`self.iTimesInteractedWith`)
    (:`  `
      (`TextRenderComponent.K2_SetText` (`self.Txt_InteractionNumber`) (`|FormatText` "{ num} TIMES" (`self.iTimesInteractedWith`))))))

(event `self.Sphere.OnComponentBeginOverlap`
  (params (OverlappedComponent :type "PrimitiveComponent Object Reference") (OtherActor :type "Actor Object Reference") (OtherComp :type "PrimitiveComponent Object Reference") (OtherBodyIndex :type Integer) (bFromSweep :type Boolean) (SweepResult :type "HitResult Structure (by ref)"))
  (message `KFI_Interact.EnteredInteractionZone` OtherActor self)
  (`TextRenderComponent.K2_SetText` (`self.Txt_InVolume`) "YES")
  (`TextRenderComponent.SetTextRenderColor` (`self.Txt_InVolume`) (make `Color` 0 255)))

(event `self.Sphere.OnComponentEndOverlap`
  (params (OverlappedComponent :type "PrimitiveComponent Object Reference") (OtherActor :type "Actor Object Reference") (OtherComp :type "PrimitiveComponent Object Reference") (OtherBodyIndex :type Integer))
  (message `KFI_Interact.LeftInteractionZone` OtherActor self)
  (`TextRenderComponent.K2_SetText` (`self.Txt_InVolume`) "NO")
  (`TextRenderComponent.SetTextRenderColor` (`self.Txt_InVolume`) (make `Color` 0 0 255)))

(fn `UserConstructionScript`)