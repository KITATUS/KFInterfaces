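; BP_Chest is an interactable chest that toggles open and closed on each interaction request.
; A timeline plays forward or in reverse to drive a rotator lerp that swings SceneTopMesh between its closed and open rotations.
; A sphere trigger sends entered and left interaction zone messages to overlapping actors, passing the chest itself as the interactable.
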(event `self.InteractRequest`
  (params (InteractableActor :type "Actor Object Reference"))
  (bind _output_get (set `self.bOpen` (not (`self.bOpen`))))
  (if _output_get
    (bind (_direction _0_1lerp) (`Timeline|Timeline_0` :!label _label)
      (:`Update`
        (`SceneComponent.K2_SetRelativeRotation` (`self.Scene_TopMesh`) (`KismetMathLibrary.RLerp` (struct) (struct :`Pitch` -90.0) _0_1lerp true) false false)))
    (else
      (goto _label :!via `Reverse`))))

(event `self.Sphere.OnComponentBeginOverlap`
  (params (OverlappedComponent :type "PrimitiveComponent Object Reference") (OtherActor :type "Actor Object Reference") (OtherComp :type "PrimitiveComponent Object Reference") (OtherBodyIndex :type Integer) (bFromSweep :type Boolean) (SweepResult :type "HitResult Structure (by ref)"))
  (message `KFI_Interact.EnteredInteractionZone` OtherActor self))

(event `self.Sphere.OnComponentEndOverlap`
  (params (OverlappedComponent :type "PrimitiveComponent Object Reference") (OtherActor :type "Actor Object Reference") (OtherComp :type "PrimitiveComponent Object Reference") (OtherBodyIndex :type Integer))
  (message `KFI_Interact.LeftInteractionZone` OtherActor self))

(fn `UserConstructionScript`)